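; BP_PlayerController handles player input for BP_Character, covering look, movement, jump and pause.
; On BeginPlay it casts and caches player character 0, then forwards axis and action inputs to it.
; Movement follows the actor's forward and right vectors.
; Pause clears all widgets, toggles the game's paused state and shows either the character-owned HUD or pause menu.
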(event EventBeginPlay
  ;[1 1 1] Parameterize our custom character (As BP Character)
  (bind _asbp_character (Utilities|Casting|CastToBP_Character (Game|GetPlayerCharacter 0)))
  (Variables|Default|SetAs%20BP%20Character _asbp_character))

(event Input|ActionEvents|InputActionJumpf
  (params (Key :type Key%20Structure :default "None"))
  ;[1 1 1] Character Jumpf!
  (:Pressed
    (Character|Jump (Variables|Default|GetAs%20BP%20Character))))

(event Input|ActionEvents|InputActionPause
  (params (Key :type Key%20Structure :default "None"))
  (bind _as_bp_character (Variables|Default|GetAs%20BP%20Character))
  ;[1 1 1] Pause Game
  (:Pressed
    (Viewport|RemoveAllWidgets)
    (if (Game|IsGamePaused)
      (UserInterface|Viewport|AddtoViewport (Variables|/Game/Framework/BP_Character.BP_Character_C|GetBP_HUD _as_bp_character) 0)
      (Game|SetGamePaused false)
      (else
        (UserInterface|Viewport|AddtoViewport (Variables|/Game/Framework/BP_Character.BP_Character_C|GetPauseMenu _as_bp_character) 0)
        (Game|SetGamePaused true)))))

(event Input|AxisEvents|InputAxisLookUp/Down
  (params (AxisValue :type Float%20%28single-precision%29))
  ;[1 1 1] Character Look Around
  (Pawn|Input|AddControllerPitchInput (Variables|Default|GetAs%20BP%20Character) AxisValue))

(event Input|AxisEvents|InputAxisLookLeft/Right
  (params (AxisValue :type Float%20%28single-precision%29))
  ;[1 1 1] Character Look Around
  (Pawn|Input|AddControllerYawInput (Variables|Default|GetAs%20BP%20Character) AxisValue))

(event Input|AxisEvents|InputAxisMoveForward/Backward
  (params (AxisValue :type Float%20%28single-precision%29))
  (bind _as_bp_character (Variables|Default|GetAs%20BP%20Character))
  ;[1 1 1] Character Movement
  (Pawn|Input|AddMovementInput _as_bp_character (Transformation|GetActorForwardVector _as_bp_character) AxisValue false))

(event Input|AxisEvents|InputAxisMoveLeft/Right
  (params (AxisValue :type Float%20%28single-precision%29))
  (bind _as_bp_character (Variables|Default|GetAs%20BP%20Character))
  ;[1 1 1] Character Movement
  (Pawn|Input|AddMovementInput _as_bp_character (Transformation|GetActorRightVector _as_bp_character) AxisValue false))

(fn ConstructionScript)
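; BP_Orb is a collectible orb actor that wobbles in place until the player character picks it up.
; A looping one-second timer randomly nudges the RotatingMovement component's rotation rate and pivot, clamped to set ranges, for erratic motion.
; On overlap with BP_Character it increments OrbsCollected, briefly enables the collected tint flag, then destroys itself after the delay.
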(event Custom|Update%20Rotation
  (bind _rotatingmovement (Variables|Default|GetRotatingMovement))
  (Variables|/Script/Engine.RotatingMovementComponent|SetRotationRate _rotatingmovement (Math|Rotator|MakeRotator (Math|Float|Max(Float) (Math|Float|Min(Float) (+ (.roll (Variables|/Script/Engine.RotatingMovementComponent|GetRotationRate _rotatingmovement)) (Math|Random|RandomFloatinRange -3e+01 3e+01)) 3e+02) -3e+02) (Math|Float|Max(Float) (Math|Float|Min(Float) (+ (.pitch (Variables|/Script/Engine.RotatingMovementComponent|GetRotationRate _rotatingmovement)) (Math|Random|RandomFloatinRange -3e+01 3e+01)) 3e+02) -3e+02) (Math|Float|Max(Float) (Math|Float|Min(Float) (+ (.yaw (Variables|/Script/Engine.RotatingMovementComponent|GetRotationRate _rotatingmovement)) (Math|Random|RandomFloatinRange -3e+01 3e+01)) 3e+02) -3e+02)))
  (Variables|/Script/Engine.RotatingMovementComponent|SetPivotTranslation _rotatingmovement (Math|Vector|MakeVector (Math|Float|Max(Float) (Math|Float|Min(Float) (+ (.x (Variables|/Script/Engine.RotatingMovementComponent|GetPivotTranslation _rotatingmovement)) (Math|Random|RandomFloatinRange -2.0 2.0)) 2e+01) -2e+01) (Math|Float|Max(Float) (Math|Float|Min(Float) (+ (.y (Variables|/Script/Engine.RotatingMovementComponent|GetPivotTranslation _rotatingmovement)) (Math|Random|RandomFloatinRange -2.0 2.0)) 2e+01) -2e+01) (Math|Float|Max(Float) (Math|Float|Min(Float) (+ (.z (Variables|/Script/Engine.RotatingMovementComponent|GetPivotTranslation _rotatingmovement)) (Math|Random|RandomFloatinRange -0.5 0.5)) 3e+01) 1e+01))))

(event Collision|EventActorBeginOverlap
  (params (OtherActor :type Actor%20Object%20Reference))
  ;[1 1 1] Collect Orb
  (bind _asbp_character (Utilities|Casting|CastToBP_Character OtherActor))
  (Variables|/Game/Framework/BP_Character.BP_Character_C|SetOrbsCollected _asbp_character (+ (Variables|/Game/Framework/BP_Character.BP_Character_C|GetOrbsCollected _asbp_character) 1))
  (Variables|/Game/Framework/BP_Character.BP_Character_C|SetShowOrbCollectedTint _asbp_character true)
  (Utilities|FlowControl|Delay 0.3)
  (Variables|/Game/Framework/BP_Character.BP_Character_C|SetShowOrbCollectedTint _asbp_character false)
  (Actor|DestroyActor))

(event EventBeginPlay
  (Utilities|Time|SetTimerbyEvent (delegate Custom|Update%20Rotation) 1.0 true))

(fn ConstructionScript)
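; BP_PillarLight is a light actor that flickers at random from BeginPlay onward.
; An endless latent loop waits on a Delay set by the product of two random values, giving irregular timing.
; Each pass picks a random intensity across a very wide range for the SpotLight and gives the PointLight a scaled-down fraction of it, so both change together.
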(event EventBeginPlay
  (bind _returnvalue (Math|Random|RandomFloatinRange 0.2 1.3))
  (Utilities|FlowControl|Delay (* _returnvalue _returnvalue) :!label _label)
  (Variables|Default|SetOverallIntensity (Math|Random|RandomFloatinRange 2e+02 2.8e+05))
  (Rendering|Components|Light|SetIntensity (Variables|Default|GetSpotLight) (Variables|Default|GetOverallIntensity))
  (Rendering|Components|Light|SetIntensity (Variables|Default|GetPointLight) (/ (Variables|Default|GetOverallIntensity) 2e+02))
  (goto _label))

(fn ConstructionScript)
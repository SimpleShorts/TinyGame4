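; End-of-level door actor that swings open on a timeline when the player presses UseObject inside its collision volume.
; Overlap with BP_Character sets a screen message based on whether three orbs are collected and enables input; leaving clears both.
; Input is enabled regardless of orb count, and the open action does not check it.
; A DoOnce limits opening to one yaw rotation from the door's initial rotation.
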(event OnComponentBeginOverlap(DoorCollision)
  (params (OverlappedComponent :type Primitive%20Component%20Object%20Reference) (OtherActor :type Actor%20Object%20Reference) (OtherComp :type Primitive%20Component%20Object%20Reference) (OtherBodyIndex :type Integer) (bFromSweep :type Boolean) (SweepResult :type Hit%20Result%20Structure%20%28by%20ref%29))
  ;[1 1 1] Enable / Disable Input on Door
  (bind _asbp_character (Utilities|Casting|CastToBP_Character OtherActor))
  (if (== (Variables|/Game/Framework/BP_Character.BP_Character_C|GetOrbsCollected _asbp_character) 3)
    (Variables|/Game/Framework/BP_Character.BP_Character_C|SetScreenMessage _asbp_character "Press F to open door!")
    (else
      (Variables|/Game/Framework/BP_Character.BP_Character_C|SetScreenMessage _asbp_character "You must collect all orbs to unlock door!")))
  (Input|EnableInput (Game|GetPlayerController 0)))

(event OnComponentEndOverlap(DoorCollision)
  (params (OverlappedComponent :type Primitive%20Component%20Object%20Reference) (OtherActor :type Actor%20Object%20Reference) (OtherComp :type Primitive%20Component%20Object%20Reference) (OtherBodyIndex :type Integer))
  ;[1 1 1] Enable / Disable Input on Door
  (bind _asbp_character (Utilities|Casting|CastToBP_Character OtherActor))
  (Variables|/Game/Framework/BP_Character.BP_Character_C|SetScreenMessage _asbp_character "")
  (Input|DisableInput (Game|GetPlayerController 0)))

(event EventBeginPlay)

(event Input|ActionEvents|InputActionUseObject
  (params (Key :type Key%20Structure :default "None"))
  ;[1 1 1] Open Door
  (:Pressed
    (Utilities|FlowControl|DoOnce false
      (:Completed
        (bind _output_get (Variables|Default|SetInitialDoorRotation (Transformation|GetActorRotation)))
        (bind _opendoormovement (Timeline|OpenDoorTimeline Play)
          (:Update
            (Transformation|SetActorRotation (Math|Rotator|MakeRotator (.Roll (Math|Rotator|BreakRotator _output_get)) (.Pitch (Math|Rotator|BreakRotator _output_get)) (- (.Yaw (Math|Rotator|BreakRotator _output_get)) _opendoormovement)))))))))

(fn ConstructionScript)
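; BP_Character is a character Blueprint that tracks health and ends the game when it runs out.
; AnyDamage passes through a DoOnce, subtracts damage from Health, then prints the remaining value and resets after a short delay, so hits in that window are ignored.
; When Health reaches roughly zero, the GameOver event quits the game and the gate stays closed.
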(event Custom|Game%20Over
  (Game|QuitGame 0 "Quit" false))

(event EventBeginPlay)

(event Collision|EventActorBeginOverlap
  (params (OtherActor :type Actor%20Object%20Reference)))

(event EventTick
  (params (DeltaSeconds :type Float%20%28single-precision%29)))

(event Game|Damage|EventAnyDamage
  (params (Damage :type Float%20%28single-precision%29) (DamageType :type Damage%20Type%20Object%20Reference) (InstigatedBy :type Controller%20Object%20Reference) (DamageCauser :type Actor%20Object%20Reference))
  ;[1 1 1] Deduct Health
  (Utilities|FlowControl|DoOnce false :!label _label
    (:Completed
      (bind _output_get (Variables|Default|SetHealth (- (Variables|Default|GetHealth) Damage)))
      (if (<= _output_get 0.0001)
        (CallFunction|GameOver)
        (else
          (Development|PrintString (Utilities|String|ToString(Float) _output_get))
          (Utilities|FlowControl|Delay 0.5)
          (goto _label Reset))))))

(fn ConstructionScript)
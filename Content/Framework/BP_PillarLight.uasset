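; BP_PillarLight is a light Blueprint that flickers its SpotLight and PointLight at random for as long as it runs.
; BeginPlay starts an endless Delay loop, waiting for the product of two random values, which skews the timing toward shorter intervals.
; Each pass picks a random intensity across a wide range for the SpotLight and sets the PointLight to a fixed small fraction of it, keeping both in sync.
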(event EventBeginPlay
  (bind _returnvalue (Math|Random|RandomFloatinRange 0.2 1.5))
  (Utilities|FlowControl|Delay (* _returnvalue _returnvalue) :!label _label)
  (Variables|Default|SetNewVar (Math|Random|RandomFloatinRange 1e+03 2.8e+05))
  (Rendering|Components|Light|SetIntensity (Variables|Default|GetSpotLight) (Variables|Default|GetNewVar))
  (Rendering|Components|Light|SetIntensity (Variables|Default|GetPointLight) (/ (Variables|Default|GetNewVar) 2e+02))
  (goto _label))

(fn ConstructionScript)